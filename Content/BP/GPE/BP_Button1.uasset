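; BP_Button1 is an interactable button that activates a linked trigger node when used.
; On BeginPlay it binds its interact event and registers itself with NodeToTrigger.
; An interaction after the cooldown calls OnActivate on the node, then a timer calls OnDeActivate after TimeReset; without a reset time, no deactivation is sent.
; Tick recharges the cooldown only while the button is inactive.
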(event `self.ReceiveBeginPlay`
  (add `self.onInteract` (delegate `onInteract_Event`))
  (`Node.AddActorToList` (`self.NodeToTrigger`) self))

(event `onInteract_Event` :!signature `self.onInteract`
  (params (character :type "PuzzleCharacter Object Reference"))
  (bind _timereset (`self.TimeReset`))
  (bind _nodetotrigger (`self.NodeToTrigger`))
  (if (`self.IsActive`)
    _
    (elif (>= (`self.Cooldown`) (`self.MaxCooldown`))
      (set `self.IsActive` true)
      (if (`KismetSystemLibrary.IsValid` _nodetotrigger)
        (`LogicNode.OnActivate` _nodetotrigger self)
        (set `self.Cooldown` 0.0)
        (if (> _timereset 0.0)
          (`KismetSystemLibrary.K2_SetTimerDelegate` (delegate `CustomEvent`) _timereset)
          (else
            (set `self.IsActive` false)))))))

(event `CustomEvent`
  (`Node.OnDeActivate` (`self.NodeToTrigger`) self)
  (set `self.IsActive` false))

(event `self.ReceiveTick`
  (params (DeltaSeconds :type "Float (single-precision)"))
  (if (>= (`self.Cooldown`) (`self.MaxCooldown`))
    _
    (elif (not (`self.IsActive`))
      (set `self.Cooldown` (+ (`self.Cooldown`) DeltaSeconds)))))

(fn `UserConstructionScript`)